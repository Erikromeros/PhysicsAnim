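; BP_Hint is a hint Blueprint in the Horse content that displays a Widget component.
; At BeginPlay it only turns off the widget's shadow casting.
; An unconnected graph, which never runs, holds authority and role checks meant to show the widget only to the owning player, as a workaround for "Only Owner See" failing on UE5 widgets.
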(event `self.ReceiveBeginPlay`
  (`PrimitiveComponent.SetCastShadow` (`self.Widget`) false))

(fn `UserConstructionScript`)