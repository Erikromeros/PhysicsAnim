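; Player rider character for the Taming minigame, with crouching and a grappling hook.
; Left mouse traces from the follow camera; a hit stores the grab point, switches movement to Flying and shows the cable.
; While grappling, Tick pins the cable end to that point and applies force toward it, blended with sideways move input for steering.
; Releasing the button hides the cable and sets movement to Falling.
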(event `Key|Nine`
  (params (Key :type "Key Structure"))
  ; Crouching mechanic
  (:`Pressed`
    (`self.Crouch`))
  (:`Released`
    (`self.UnCrouch`)))

(event `Key|LeftMouseButton`
  (params (Key :type "Key Structure"))
  (bind _followcamera (`self.FollowCamera`))
  (bind _returnvalue (`SceneComponent.K2_GetComponentLocation` _followcamera))
  ; Grappling mechanic
  (:`Pressed`
    (bind (_outhit _returnvalue_2) (`KismetSystemLibrary.LineTraceSingle` :`Start` _returnvalue :`End` (+ _returnvalue (* (`KismetMathLibrary.GetForwardVector` (`SceneComponent.K2_GetComponentRotation` _followcamera)) 4000.0)) :`TraceChannel` "TraceTypeQuery1" :`DrawDebugType` "ForDuration"))
    (if _returnvalue_2
      (set `self.GrabPoint` (`.ImpactPoint` (`GameplayStatics.BreakHitResult` _outhit)))
      (set `self.IsGrappling` true)
      (`CharacterMovementComponent.SetMovementMode` (`self.CharacterMovement`) "MOVE_Flying" 0)
      (`SceneComponent.SetVisibility` (`self.Cable`) true false)))
  (:`Released`
    (set `self.IsGrappling` false)
    (`CharacterMovementComponent.SetMovementMode` (`self.CharacterMovement`) "MOVE_Falling" 0)
    (`SceneComponent.SetVisibility` (`self.Cable`) false false)))

(event `self.ReceiveTick`
  (params (DeltaSeconds :type "Float (single-precision)"))
  (if (`self.IsGrappling`)
    (set `CableComponent.EndLocation` (`KismetMathLibrary.InverseTransformLocation` (`self.GetTransform`) (`self.GrabPoint`)) (`self.Cable`))
    (`CharacterMovementComponent.AddForce` (`self.CharacterMovement`) (* (`KismetMathLibrary.Normal` (+ (`KismetMathLibrary.GetDirectionUnitVector` (`self.K2_GetActorLocation`) (`self.GrabPoint`)) (* (* (`self.GetActorRightVector`) (`|GetInputActionValue`)) 0.7))) 250000.0))))

(fn `UserConstructionScript`
  (`parent.UserConstructionScript`))